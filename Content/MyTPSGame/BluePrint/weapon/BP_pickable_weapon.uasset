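; Pickable weapon actor that shows a weapon body and magazine mesh and records its name on the player who picks it up.
; On overlap it binds to the player's BP_CP_weaponComponent events to toggle a custom-depth highlight.
; Picked writes the main or sub weapon slot, attaching to a hand socket for main, though BeginPlay marks it as sub.
; ToEnable always configures an AK47; the switch for other weapons is disconnected.
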(event `self.ReceiveBeginPlay`
  (set `self.isMainweapon` false)
  (set `self.bispickable` false)
  (`/Game/MyTPSGame/BluePrint/weapon/BPI_pickableWeapon.toEnable` (struct))
  (`KismetSystemLibrary.Delay` 2.0))

(event `self.ReceiveActorBeginOverlap`
  (params (OtherActor :type "Actor Object Reference"))
  (bind _returnvalue (`self.GetComponentByClass` OtherActor "/Game/MyTPSGame/BluePrint/weapon/BP_CP_weaponComponent.BP_CP_weaponComponent_C"))
  (add `/Game/MyTPSGame/BluePrint/weapon/BP_CP_weaponComponent.CanPick` _returnvalue (delegate `Can Pick`))
  (add `/Game/MyTPSGame/BluePrint/weapon/BP_CP_weaponComponent.CantPick` _returnvalue (delegate `Cant Pick`)))

(event `Cant Pick`
  (`PrimitiveComponent.SetRenderCustomDepth` (`self.weaponMesh`) false)
  (`PrimitiveComponent.SetRenderCustomDepth` (`self.magMesh`) false))

(event `Can Pick`
  (`PrimitiveComponent.SetRenderCustomDepth` (`self.weaponMesh`) true)
  (`PrimitiveComponent.SetRenderCustomDepth` (`self.magMesh`) true))

(event `self.ReceiveActorEndOverlap`
  (params (OtherActor :type "Actor Object Reference"))
  (bind _returnvalue (`self.GetComponentByClass` OtherActor "/Game/MyTPSGame/BluePrint/weapon/BP_CP_weaponComponent.BP_CP_weaponComponent_C"))
  (remove `/Game/MyTPSGame/BluePrint/weapon/BP_CP_weaponComponent.CanPick` _returnvalue (delegate `Can Pick`))
  (remove `/Game/MyTPSGame/BluePrint/weapon/BP_CP_weaponComponent.CantPick` _returnvalue (delegate `Cant Pick`)))

(event `/Game/MyTPSGame/BluePrint/weapon/BPI_pickableWeapon.picked`
  (params (pickerAplayer :type "/Game/MyTPSGame/BluePrint/Charactors/Player/BP_APlayer Object Reference"))
  (bind _returnvalue (`self.GetComponentByClass` pickerAplayer "/Game/MyTPSGame/BluePrint/weapon/BP_CP_weaponComponent.BP_CP_weaponComponent_C"))
  (bind _weaponname (`self.weaponName`))
  (if (`self.isMainweapon`)
    (set `/Game/MyTPSGame/BluePrint/weapon/BP_CP_weaponComponent.mainWeapon` _weaponname _returnvalue)
    (`self.K2_AttachToComponent` (`self.GetComponentByClass` pickerAplayer "/Script/Engine.StaticMeshComponent") "weapon_r_gun" "KeepRelative" "KeepRelative" "KeepRelative")
    (else
      (set `/Game/MyTPSGame/BluePrint/weapon/BP_CP_weaponComponent.subWeapon` _weaponname _returnvalue))))

(event `/Game/MyTPSGame/BluePrint/weapon/BPI_pickableWeapon.toDestory`
  (`self.K2_DestroyActor`))

(event `/Game/MyTPSGame/BluePrint/weapon/BPI_pickableWeapon.toDisable`
  (set `self.bispickable` false))

(event `/Game/MyTPSGame/BluePrint/weapon/BPI_pickableWeapon.toEnable`
  (params (weapon :type "/Game/MyTPSGame/Structs/ST_weapon Structure"))
  (`StaticMeshComponent.SetStaticMesh` (`self.weaponMesh`) "/Game/MyTPSGame/content/models/guns/AK47_Body.AK47_Body")
  (`StaticMeshComponent.SetStaticMesh` (`self.magMesh`) "/Game/MyTPSGame/content/models/guns/Ak47_Magazine.Ak47_Magazine")
  (`SceneComponent.K2_AddWorldOffset` (`self.magMesh`) (0.6 -8.0 0.0) false false)
  (set `self.weaponName` "ak"))

(fn `UserConstructionScript`)