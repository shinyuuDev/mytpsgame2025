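; BP_APlayer is the player Character Blueprint, handling Enhanced Input movement, look and jump, plus HUD setup.
; On controller change it adds the IMC_APlayer mapping context and prints a debug "Hello".
; BeginPlay creates the WBP_APlayer widget, passes it the weapon component and adds it to the viewport.
; Movement follows control yaw, look pitch is inverted, and the Interact event is an empty stub.
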(event `/Game/MyTPSGame/BluePrint/BPI_interact.interact`)

(event `self.ReceiveBeginPlay`
  (bind _asplayer_controller (cast `PlayerController` (`self.GetController` self)))
  (bind _returnvalue (`|CreateWidget` "/Game/MyTPSGame/UI/WBP_APlayer.WBP_APlayer_C" _asplayer_controller))
  (bind _output_get (set `self.PlayerWidget` _returnvalue))
  (set `/Game/MyTPSGame/UI/WBP_APlayer.componentWeapon` (`self.BP_CP_weaponComponent`) _output_get)
  (`UserWidget.AddToViewport` _returnvalue 0))

(event `self.ReceiveControllerChanged`
  (params (OldController :type "Controller Object Reference") (NewController :type "Controller Object Reference"))
  (set `self.playerController` NewController)
  (bind _asplayer_controller (cast `PlayerController` NewController))
  (`KismetSystemLibrary.PrintString` "Hello")
  (`EnhancedInputSubsystemInterface.AddMappingContext` (pcsubsystem `EnhancedInputLocalPlayerSubsystem` _asplayer_controller) "/Game/MyTPSGame/BluePrint/Charactors/Player/Player_EnhancedInput/IMC_APlayer.IMC_APlayer" 0 (struct)))

(event `EnhancedInput|/Game/MyTPSGame/BluePrint/Charactors/Player/Player_EnhancedInput/IA_APlayer_Look`
  (params (ActionValue :type "Vector2D Structure") (ElapsedSeconds :type "Float (double-precision)") (TriggeredSeconds :type "Float (double-precision)") (InputAction :type "InputAction Object Reference" :default "/Game/MyTPSGame/BluePrint/Charactors/Player/Player_EnhancedInput/IA_APlayer_Look.IA_APlayer_Look"))
  (:`Triggered`
    (`self.AddControllerYawInput` ActionValue_X)
    (`self.AddControllerPitchInput` (* ActionValue_Y -1.0))))

(event `EnhancedInput|/Game/MyTPSGame/BluePrint/Charactors/Player/Player_EnhancedInput/IA_APlayer_Move`
  (params (ActionValue :type "Vector2D Structure") (ElapsedSeconds :type "Float (double-precision)") (TriggeredSeconds :type "Float (double-precision)") (InputAction :type "InputAction Object Reference" :default "/Game/MyTPSGame/BluePrint/Charactors/Player/Player_EnhancedInput/IA_APlayer_Move.IA_APlayer_Move"))
  (bind (_returnvalue_roll _returnvalue_pitch _returnvalue_yaw) (`KismetMathLibrary.BreakRotator` (`self.GetControlRotation`)))
  (bind (_returnvalue_roll_2 _returnvalue_pitch_2 _returnvalue_yaw_2) (`KismetMathLibrary.BreakRotator` (`self.GetControlRotation`)))
  (:`Triggered`
    (`self.AddMovementInput` (`KismetMathLibrary.GetRightVector` (`KismetMathLibrary.MakeRotator` 0.0 0.0 _returnvalue_yaw)) ActionValue_X)
    (`self.AddMovementInput` (`KismetMathLibrary.GetForwardVector` (`KismetMathLibrary.MakeRotator` 0.0 0.0 _returnvalue_yaw_2)) ActionValue_Y)))

(event `EnhancedInput|/Game/MyTPSGame/BluePrint/Charactors/Player/Player_EnhancedInput/IA_APlayer_Jump`
  (params (ActionValue :type Boolean) (ElapsedSeconds :type "Float (double-precision)") (TriggeredSeconds :type "Float (double-precision)") (InputAction :type "InputAction Object Reference" :default "/Game/MyTPSGame/BluePrint/Charactors/Player/Player_EnhancedInput/IA_APlayer_Jump.IA_APlayer_Jump"))
  (:`Triggered`
    (`self.Jump`))
  (:`Completed`
    (`self.StopJumping`)))

(fn `UserConstructionScript`)